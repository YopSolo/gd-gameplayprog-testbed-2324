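; BP_BigDoor is a large door that slides vertically, sinking when opened and rising when closed.
; OpenMe and CloseMe play one Timeline forward or in reverse, lerping the actor's world Z between two fixed heights.
; Each event also plays a door sound after a short delay.
; When the Timeline finishes in either direction, a camera shake plays centered on the player character.
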(event Custom|OpenMe
  (bind _returnvalue (Transformation|GetActorLocation))
  (Utilities|FlowControl|Sequence
    (:then_0
      (bind _alpha (Timeline|Timeline PlayFromStart)
        (:Update
          (Transformation|SetActorLocation (Math|Vector|MakeVector (.x _returnvalue) (.y _returnvalue) (Math|Float|Lerp 1.5e+02 -139.0 _alpha)) false false))
        (:Finished
          (Camera|PlayWorldCameraShake "/Game/BigDoor/MyCameraShake.MyCameraShake_C" (Transformation|GetActorLocation (Game|GetPlayerCharacter 0)) 1e+02 1e+03 1e+01))))
    (:then_1
      (Utilities|FlowControl|Delay 0.8)
      (Audio|Components|Audio|Play (Variables|Default|Get029-Door06_Cue) 0.0))))

(event Custom|CloseMe
  (bind _returnvalue (Transformation|GetActorLocation))
  (Utilities|FlowControl|Sequence
    (:then_0
      (bind _alpha (Timeline|Timeline ReverseFromEnd)
        (:Update
          (Transformation|SetActorLocation (Math|Vector|MakeVector (.x _returnvalue) (.y _returnvalue) (Math|Float|Lerp 1.5e+02 -139.0 _alpha)) false false))
        (:Finished
          (Camera|PlayWorldCameraShake "/Game/BigDoor/MyCameraShake.MyCameraShake_C" (Transformation|GetActorLocation (Game|GetPlayerCharacter 0)) 1e+02 1e+03 1e+01))))
    (:then_1
      (Utilities|FlowControl|Delay 0.2)
      (Audio|Components|Audio|Play (Variables|Default|Get029-Door06_Cue) 0.0))))

(fn ConstructionScript)